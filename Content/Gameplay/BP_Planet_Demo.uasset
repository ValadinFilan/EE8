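; Demo planet actor that showcases each planet look defined in a data table while spinning in place.
; After an initial delay, BeginPlay reads the row names, then a delayed loop steps through them every few seconds without wrapping.
; Each found row sets the planet and cloud sphere materials and prints its name.
; Tick adds a fixed yaw each frame, so spin speed depends on frame rate.
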(event `self.ReceiveBeginPlay`
  (bind _dt (`self.DT`))
  (`parent.ReceiveBeginPlay`)
  ;[1 1 1] CreateCosmetic Implementation
  (`KismetSystemLibrary.Delay` 5.0)
  (bind _outrownames (`DataTableFunctionLibrary.GetDataTableRowNames` _dt))
  (`KismetSystemLibrary.Delay` 5.0 :!label _label)
  (bind _output (`|GetArrayItem` _outrownames (`self.NewVar_0`)))
  (bind _returnvalue (`|GetDataTableRow` _dt _output)
    (:`then`
      (bind (_description _planet_material _clouds_material) (break `/Game/Misc/PlanetStruct` _returnvalue))
      (`PrimitiveComponent.SetMaterial` (`self.ObjectMesh`) 0 _planet_material)
      (`PrimitiveComponent.SetMaterial` (`self.CloudSphere`) 0 _clouds_material)
      (`KismetSystemLibrary.PrintString` (`KismetStringLibrary.Conv_NameToString` _output))
      (set `self.NewVar_0` (+ (`self.NewVar_0`) 1))
      (goto _label))))

(event `self.ReceiveTick`
  (params (DeltaSeconds :type "Float (single-precision)"))
  (`self.K2_AddActorWorldRotation` (struct :`Yaw` 0.4)))

(fn `UserConstructionScript`
  (`parent.UserConstructionScript`))