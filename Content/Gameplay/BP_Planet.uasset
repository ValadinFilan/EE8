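; Planet actor that gives itself a randomized look for its surface and cloud layer.
; Its CreateCosmetic override picks a random data table row through a random stream and applies that row's planet and cloud materials to ObjectMesh and CloudSphere.
; The parent cosmetic call and a planet widget creation are left disconnected, so clicking the planet does nothing in this graph.
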(event `self.ReceiveBeginPlay`)

(event `self.CreateCosmetic`
  (bind _dt (`self.DT`))
  ;[1 1 1] CreateCosmetic Implementation
  (bind _outrownames (`DataTableFunctionLibrary.GetDataTableRowNames` _dt))
  (bind _returnvalue (`|GetDataTableRow` _dt (`|GetArrayItem` _outrownames (`KismetMathLibrary.RandomIntegerInRangeFromStream` 0 (- (`KismetArrayLibrary.Array_Length` _outrownames) 1) (`self.RStream`))))
    (:`then`
      (bind (_description _planet_material _clouds_material) (break `/Game/Misc/PlanetStruct` _returnvalue))
      (`PrimitiveComponent.SetMaterial` (`self.ObjectMesh`) 0 _planet_material)
      (`PrimitiveComponent.SetMaterial` (`self.CloudSphere`) 0 _clouds_material))))

(event `self.ReceiveActorOnClicked`
  (params (ButtonPressed :type "Key Structure")))

(fn `UserConstructionScript`)